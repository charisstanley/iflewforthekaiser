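; BP_EnemySpawner is an actor that keeps spawning BP_ParentEnemy at one of three point components.
; BeginPlay starts a looping timer, stored as EnemySpawnerTimer, with an interval randomized once between half a second and two seconds.
; Each tick of that timer picks one of the three points at random, spawns the enemy at its world transform and prints a debug message.
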(event Custom|Enemy%20Spawn
  (Game|SpawnActorfromClass "/Game/_Blueprints/Enemy/BP_ParentEnemy.BP_ParentEnemy_C" (Utilities|Select :Index (Math|Random|RandomIntegerinRange 0 2) :Option%200 (Transformation|GetWorldTransform (Variables|Default|GetPoint_01)) :Option%201 (Transformation|GetWorldTransform (Variables|Default|GetPoint_02)) :Option%202 (Transformation|GetWorldTransform (Variables|Default|GetPoint_03))) "Undefined" 0 0)
  (Development|PrintString "Spawning"))

(event EventBeginPlay
  (bind _returnvalue (Utilities|Time|SetTimerbyEvent (delegate Custom|Enemy%20Spawn) (Math|Random|RandomFloatinRange 0.5 2.0) true))
  (Variables|Default|SetEnemySpawnerTimer _returnvalue))

(fn ConstructionScript)