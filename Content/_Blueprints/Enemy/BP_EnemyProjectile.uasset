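; BP_EnemyProjectile is an enemy projectile actor that damages the player on contact.
; On BeginPlay it sets the ProjectileMovement initial speed from its InitialSpeed variable and caps max speed at a multiple of that.
; When its Box component overlaps a BP_Player, it applies Damage to that player and destroys itself, ignoring any other actor.
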(event OnComponentBeginOverlap(Box)
  (params (OverlappedComponent :type Primitive%20Component%20Object%20Reference) (OtherActor :type Actor%20Object%20Reference) (OtherComp :type Primitive%20Component%20Object%20Reference) (OtherBodyIndex :type Integer) (bFromSweep :type Boolean) (SweepResult :type Hit%20Result%20Structure%20%28by%20ref%29))
  (bind _asbp_player (Utilities|Casting|CastToBP_Player OtherActor))
  (bind _output_get (Variables|Default|SetPlayer%20Pawn _asbp_player))
  (Game|Damage|ApplyDamage _output_get (Math|Conversions|ToFloat(Integer) (Variables|Default|GetDamage)) 0 0)
  (Actor|DestroyActor))

(event EventBeginPlay
  (bind _projectilemovement (Variables|Default|GetProjectileMovement))
  (Variables|/Script/Engine.ProjectileMovementComponent|SetInitialSpeed _projectilemovement (Variables|Default|GetInitialSpeed))
  (Variables|/Script/Engine.ProjectileMovementComponent|SetMaxSpeed _projectilemovement (* (Variables|Default|GetInitialSpeed) 1.5)))

(fn ConstructionScript)