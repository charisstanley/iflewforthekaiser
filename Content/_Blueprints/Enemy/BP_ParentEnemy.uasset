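; BP_ParentEnemy is an enemy, apparently a base class, that shoots projectiles when its sight trace is blocked.
; Each Tick, a debug-drawn line trace along a fixed SitesDistance offset unpauses or pauses a looping Shoot timer; any blocking hit counts as seeing the player.
; Damage lowers Health; a hit arriving at zero or below fires the OnDeath dispatcher, which awards Points through PlayerCombatController and destroys the actor.
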(event Custom|OnDeath_Event
  (params (Player%20Combat%20Controller :type PC%20Combat%20Object%20Reference))
  (Default|ScoreUpdate Player%20Combat%20Controller (Variables|Default|GetPoints))
  (CallFunction|Death))

(event Custom|OnTakeAnyDamage_Event
  (params (DamagedActor :type Actor%20Object%20Reference) (Damage :type Float%20%28single-precision%29) (DamageType :type Damage%20Type%20Object%20Reference) (InstigatedBy :type Controller%20Object%20Reference) (DamageCauser :type Actor%20Object%20Reference))
  (if (> (Variables|Default|GetHealth) 0)
    (Variables|Default|SetHealth (Math|Float|Truncate (- (Variables|Default|GetHealth) Damage)))
    (Development|PrintString "Hit")
    (else
      (Default|CallOnDeath (Variables|Default|GetPlayer%20Combat%20Controller)))))

(event Custom|Shoot
  (Game|SpawnActorfromClass "/Game/_Blueprints/Enemy/BP_EnemyProjectile.BP_EnemyProjectile_C" (Transformation|GetWorldTransform (Variables|Default|GetScene)) "Undefined" 0 0))

(event EventBeginPlay
  (EventDispatchers|BindEventtoOnDeath (delegate Custom|OnDeath_Event))
  (EventDispatchers|AssignOnTakeAnyDamage (delegate Custom|OnTakeAnyDamage_Event))
  (bind _returnvalue (Utilities|Time|SetTimerbyEvent (delegate Custom|Shoot) 0.5 true))
  (bind _output_get (Variables|Default|SetShootingTimer _returnvalue))
  (Utilities|Time|PauseTimerbyHandle _output_get))

(event EventTick
  (params (DeltaSeconds :type Float%20%28single-precision%29))
  (CallFunction|CheckforPlayerSites))

(fn ConstructionScript)

(fn Death
  (Actor|DestroyActor))

(fn CheckforPlayerSites
  (bind _scene (Variables|Default|GetScene))
  (bind _returnvalue (Transformation|GetWorldLocation _scene))
  (bind _outhit (Collision|LineTraceByChannel _returnvalue (+ _returnvalue (Variables|Default|GetSitesDistance)) "TraceTypeQuery3" false 0 "ForDuration"))
  (if (.bBlockingHit (Collision|BreakHitResult _outhit))
    (bind _output_get (Variables|Default|SetHit%20Actor (.HitActor (Collision|BreakHitResult _outhit))))
    (if (== (.HitActor (Collision|BreakHitResult _outhit)) _output_get)
      (Development|PrintString "I See YOU" true true "(R=0.000000,G=1.000000,B=0.209901,A=1.000000)")
      (Variables|Default|SetHit%20Actor 0)
      (Utilities|Time|UnpauseTimerbyHandle (Variables|Default|GetShootingTimer))
      (return true)
      (else
        _)))
  (Variables|Default|SetHit%20Actor 0)
  (Utilities|Time|PauseTimerbyHandle (Variables|Default|GetShootingTimer))
  (return false))