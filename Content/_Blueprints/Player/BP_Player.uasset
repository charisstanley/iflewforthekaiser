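; BP_Player is the player-controlled actor for a combat mode, handling movement, shooting and health.
; MoveRight and MoveForward axes share one normalized, swept world offset on the X-Z plane, scaled by speed and delta time.
; Fire spawns BP_BasicProjectile at the Gun transform, passing in the PC_Combat controller.
; Damage reduces Health, and a hit received at zero or below tells GM_Combat to update game over.
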(event Custom|OnTakeAnyDamage_Event
  (params (DamagedActor :type Actor%20Object%20Reference) (Damage :type Float%20%28single-precision%29) (DamageType :type Damage%20Type%20Object%20Reference) (InstigatedBy :type Controller%20Object%20Reference) (DamageCauser :type Actor%20Object%20Reference))
  (if (> (Variables|Default|GetHealth) 0)
    (Variables|Default|SetHealth (Math|Float|Truncate (- (Variables|Default|GetHealth) Damage)))
    (else
      (bind _asgm_combat (Utilities|Casting|CastToGM_Combat (Game|GetGameMode)))
      (Default|CallUpdateGameOver _asgm_combat)
      (Development|PrintString "Gameover" true true "(R=1.000000,G=0.753866,B=0.000000,A=1.000000)"))))

(event EventBeginPlay
  (EventDispatchers|AssignOnTakeAnyDamage (delegate Custom|OnTakeAnyDamage_Event)))

(event Input|ActionEvents|InputActionFire
  (params (Key :type Key%20Structure :default "None"))
  (:Pressed
    (Variables|Default|SetIsFiring? true)
    (Game|SpawnActorfromClass "/Game/_Blueprints/Player/BP_BasicProjectile.BP_BasicProjectile_C" (Transformation|GetWorldTransform (Variables|Default|GetGun)) "Undefined" 0 (.AsPC%20Combat (Utilities|Casting|CastToPC_Combat (Game|GetPlayerController 0))) 0)
    (Development|PrintString "Pew Pew" true true "(R=0.700000,G=0.000000,B=0.000000,A=1.000000)"))
  (:Released
    (Variables|Default|SetIsFiring? false)))

(event Input|AxisEvents|InputAxisMoveRight
  (params (AxisValue :type Float%20%28single-precision%29))
  (Variables|Default|SetMoveRight AxisValue)
  (Transformation|AddActorWorldOffset self (* (Math|Vector|Normalize (Math|Vector|MakeVector (Variables|Default|GetMoveRight) 0.0 (Variables|Default|GetMoveForward))) (* (Utilities|Time|GetWorldDeltaSeconds) (Variables|Default|GetMovementSpeed))) true))

(event Input|AxisEvents|InputAxisMoveForward
  (params (AxisValue :type Float%20%28single-precision%29))
  (Variables|Default|SetMoveForward AxisValue)
  (Transformation|AddActorWorldOffset self (* (Math|Vector|Normalize (Math|Vector|MakeVector (Variables|Default|GetMoveRight) 0.0 (Variables|Default|GetMoveForward))) (* (Utilities|Time|GetWorldDeltaSeconds) (Variables|Default|GetMovementSpeed))) true))

(fn ConstructionScript)