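; GM_Combat is the combat game mode, which shows the game over and victory screens.
; On BeginPlay it sets game-only input and binds handlers to the UpdateGameOver and UpdateScore events.
; The game over handler, guarded by DoOnce, and the unguarded score handler, which shows victory without checking a score, each add their widget to the viewport, pause the game and show the PC_Combat mouse cursor.
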(event Custom|UpdateGameOver_Event
  (params (Player%20Controller :type PC%20Combat%20Object%20Reference))
  (Utilities|FlowControl|DoOnce false
    (:Completed
      (bind _returnvalue (UserInterface|CreateWidget "/Game/_UI/BPW_GameOverScreen.BPW_GameOverScreen_C" Player%20Controller))
      (UserInterface|Viewport|AddtoViewport _returnvalue 0)
      (Game|SetGamePaused true)
      (Variables|/Script/Engine.PlayerController|SetbShowMouseCursor (.AsPC%20Combat (Utilities|Casting|CastToPC_Combat (Game|GetPlayerController 0))) true))))

(event Custom|UpdateScore_Event
  (params (Player%20Controller%20Reference :type PC%20Combat%20Object%20Reference))
  (bind _returnvalue (UserInterface|CreateWidget "/Game/_UI/BPW_VictoryScreen.BPW_VictoryScreen_C"))
  (bind _output_get (Variables|Default|SetBPW_VictoryScreen _returnvalue))
  (UserInterface|Viewport|AddtoViewport _output_get 0)
  (Game|SetGamePaused true)
  (Variables|/Script/Engine.PlayerController|SetbShowMouseCursor (.AsPC%20Combat (Utilities|Casting|CastToPC_Combat (Game|GetPlayerController 0))) true))

(event EventBeginPlay
  (Input|SetInputModeGameOnly (.AsPC%20Combat (Utilities|Casting|CastToPC_Combat (Game|GetPlayerController 0))) false)
  (EventDispatchers|BindEventtoUpdateGameOver (delegate Custom|UpdateGameOver_Event))
  (EventDispatchers|BindEventtoUpdateScore (delegate Custom|UpdateScore_Event)))

(event EventTick
  (params (DeltaSeconds :type Float%20%28single-precision%29)))

(fn ConstructionScript)