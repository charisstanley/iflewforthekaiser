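; Player controller for combat that tracks score and handles the pause menu.
; A score event bound on BeginPlay accumulates points and notifies GM_Combat on each update where the total meets or exceeds the level-clear threshold.
; The Pause input toggles game pause via a boolean, switching input mode and mouse cursor and creating or removing the BPW_PauseMenu widget.
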(event Custom|ScoreUpdate
  (params (ScoreUpdate :type Integer))
  (bind _output_get (Variables|Default|SetScore (+ (Variables|Default|GetScore) ScoreUpdate)))
  (if (>= _output_get (Variables|Default|GetLevelClearScore))
    (Default|CallUpdateScore (.AsGM%20Combat (Utilities|Casting|CastToGM_Combat (Game|GetGameMode))) self)))

(event Custom|UnpauseGame
  (Variables|Default|SetisGamePaused? false)
  (Game|SetGamePaused false)
  (Variables|Default|SetbShowMouseCursor false)
  (Input|SetInputModeGameOnly self false)
  (if (Widget|IsVisible (Variables|Default|GetBPW_PauseMenu))
    (Widget|RemovefromParent (Variables|Default|GetBPW_PauseMenu))))

(event Custom|PauseGame
  (Variables|Default|SetisGamePaused? true)
  (Game|SetGamePaused true)
  (Variables|Default|SetbShowMouseCursor true)
  (bind _returnvalue (UserInterface|CreateWidget "/Game/_UI/BPW_PauseMenu.BPW_PauseMenu_C"))
  (bind _output_get (Variables|Default|SetBPW_PauseMenu _returnvalue))
  (UserInterface|Viewport|AddtoViewport _output_get 0)
  (Input|SetInputModeGameandUI self (Variables|Default|GetBPW_PauseMenu) "LockInFullscreen" true false))

(event EventBeginPlay
  (EventDispatchers|BindEventtoEDScoreUpdate (delegate Custom|ScoreUpdate)))

(event Input|ActionEvents|InputActionPause
  (params (Key :type Key%20Structure :default "None"))
  (:Pressed
    (Utilities|FlowControl|FlipFlop
      (:A
        _)
      (:B
        _))
    (if (Variables|Default|GetisGamePaused?)
      (CallFunction|UnpauseGame)
      (else
        (CallFunction|PauseGame)))))

(fn ConstructionScript)